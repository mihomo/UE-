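; Player controller for BP_Player that handles movement, look, view switching and firing.
; Move and look input only act while the pawn's ThirdView flag is off.
; Change_View flips that flag, toggles both cameras and the mouse cursor, and on leaving third view clears any open tower attribute UI with its floor box.
; Attack drives a Gate and Delay loop that spawns bullets at the pawn's FireSpeed interval until released.
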(event `InputAxis|MoveForward`
  (params (AxisValue :type "Float (single-precision)")))

(event `InputAxis|MoveRight`
  (params (AxisValue :type "Float (single-precision)")))

(event `InputAxis|MoveForward` :overrideparent false
  (params (AxisValue :type "Float (single-precision)"))
  ;[1 1 1] 移动
  (if (not (`/Game/Item/BP_Player.Third_View?` (cast `/Game/Item/BP_Player` (`self.K2_GetPawn`) :!pure true)))
    (`Pawn.AddMovementInput` (`self.K2_GetPawn`) (`KismetMathLibrary.GetForwardVector` (`self.GetControlRotation`)) AxisValue false)))

(event `InputAxis|MoveRight` :overrideparent false
  (params (AxisValue :type "Float (single-precision)"))
  ;[1 1 1] 移动
  (if (not (`/Game/Item/BP_Player.Third_View?` (cast `/Game/Item/BP_Player` (`self.K2_GetPawn`) :!pure true)))
    (`Pawn.AddMovementInput` (`self.K2_GetPawn`) (`KismetMathLibrary.GetRightVector` (`self.GetControlRotation`)) AxisValue false)))

(event `InputAxis|Turn` :overrideparent false
  (params (AxisValue :type "Float (single-precision)"))
  (bind _asbp_player (cast `/Game/Item/BP_Player` (`self.K2_GetPawn`) :!pure true))
  ;[1 1 1] 旋转
  (if (not (`/Game/Item/BP_Player.Third_View?` _asbp_player)) :!label _label
    (`|ExecutionSequence`
      (:`then_0`
        (`Pawn.AddControllerYawInput` _asbp_player AxisValue))
      (:`then_1`
        (`Pawn.AddControllerPitchInput` _asbp_player (stale `InputAxis|LookUp` AxisValue))))))

(event `InputAxis|LookUp` :overrideparent false
  (params (AxisValue :type "Float (single-precision)"))
  ;[1 1 1] 旋转
  (goto _label))

(event `InputAction|Change_View`
  (params (Key :type "Key Structure"))
  (bind _asbp_player (cast `/Game/Item/BP_Player` (`self.K2_GetPawn`) :!pure true))
  (bind _right_ui (`/Game/Item/BP_Player.Right UI` (cast `/Game/Item/BP_Player` (`GameplayStatics.GetPlayerPawn` 0) :!pure true)))
  ;[1 1 1] 转换视角
  (:`Pressed`
    (if (`/Game/Item/BP_Player.Third_View?` _asbp_player)
      (set `/Game/Item/BP_Player.Third_View?` false _asbp_player)
      (`ActorComponent.ToggleActive` (`/Game/Item/BP_Player.Camera1` _asbp_player))
      (`ActorComponent.ToggleActive` (`/Game/Item/BP_Player.Camera` _asbp_player))
      (set `self.bShowMouseCursor` false)
      (`/Engine/EditorBlueprintResources/StandardMacros.IsValid` _right_ui
        (:`Is Valid`
          (`/Game/Item/ItemBase/TowerFloorBase.switch Show_Box` (`/Game/UI/TowerAtrributeUI.RelateTowerFloor` (cast `/Game/UI/TowerAtrributeUI` _right_ui :!pure true)))
          (`/Game/Blueprint/Gameplay/BP_TestGameInstance.Clear UI` (cast `/Game/Blueprint/Gameplay/BP_TestGameInstance` (`GameplayStatics.GetGameInstance`) :!pure true) _right_ui)))
      (else
        (set `/Game/Item/BP_Player.Third_View?` true _asbp_player)
        (`ActorComponent.ToggleActive` (`/Game/Item/BP_Player.Camera1` _asbp_player))
        (`ActorComponent.ToggleActive` (`/Game/Item/BP_Player.Camera` _asbp_player))
        (set `self.bShowMouseCursor` true)))))

(event `InputAction|Attack`
  (params (Key :type "Key Structure"))
  (bind _asbp_player (cast `/Game/Item/BP_Player` (`self.K2_GetPawn`) :!pure true))
  ;[1 1 1] 攻击
  (:`Pressed`
    (`|ExecutionSequence`
      (:`then_0`
        (goto _label_2 :!via `Open`))
      (:`then_1`
        (`/Engine/EditorBlueprintResources/StandardMacros.Gate` true :!label _label_2
          (:`Exit`
            (`/Game/Item/BP_Player.Spawn Buttle` _asbp_player)
            (`KismetSystemLibrary.Delay` (`/Game/Item/BP_Player.Fire Speed` _asbp_player))
            (goto _label_2))))))
  (:`Released`
    (goto _label_2 :!via `Close`)))

(fn `UserConstructionScript`)