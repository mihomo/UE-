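; BP_TestGameState is the game state that tracks TPS resources, enemy count and HP, and decides victory and defeat.
; ChangeAtrribute applies deltas to those values, and HP's OnRep pauses into the defeat UI at zero or below.
; Tick pauses into the win UI once 210 seconds of main-level time pass with no enemies left.
; BeginPlay uses timed delays to switch the player's ambient music track twice.
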(event `Change Atrribute`
  (params (`Change TPSResourcces` :type Integer) (`Change EnemyCount` :type Integer) (`Change HP` :type Integer) (NewParam4 :type Boolean) (NewParam5 :type Boolean))
  ;[1 1 1] 更改属性
  (set `self.TPS Resources` (+ (`self.TPS Resources`) `Change TPSResourcces`))
  (set `self.Enemy Count` (+ (`self.Enemy Count`) `Change EnemyCount`))
  (set `self.HP` (+ (`self.HP`) `Change HP`)))

(event `self.ReceiveBeginPlay`
  (bind _audio_surroundings (`/Game/Item/BP_Player.Audio_Surroundings` (cast `/Game/Item/BP_Player` (`GameplayStatics.GetPlayerPawn` 0) :!pure true)))
  (bind _audio_surroundings_2 (`/Game/Item/BP_Player.Audio_Surroundings` (cast `/Game/Item/BP_Player` (`GameplayStatics.GetPlayerPawn` 0) :!pure true)))
  ;[1 1 1] 敌人生成进程
  (`KismetSystemLibrary.Delay` 76.0)
  (`AudioComponent.SetSound` _audio_surroundings "/Game/Music/Dreaming-at-Altitude.Dreaming-at-Altitude")
  (`AudioComponent.Play` _audio_surroundings 0.0)
  (`KismetSystemLibrary.Delay` 76.0)
  (`AudioComponent.SetSound` _audio_surroundings_2 "/Game/Music/Into-Battle.Into-Battle")
  (`AudioComponent.Play` _audio_surroundings_2 0.0)
  (`KismetSystemLibrary.Delay` 56.0))

(event `self.ReceiveTick`
  (params (DeltaSeconds :type "Float (single-precision)"))
  ;[1 1 1] 游戏胜利判定
  (if (>= (`self.EnterMainLevelGameTime`) 210)
    (if (<= (`self.Enemy Count`) 0)
      (`GameplayStatics.SetGamePaused` true)
      (`/Game/Blueprint/Gameplay/BP_TestGameInstance.Win UI` (cast `/Game/Blueprint/Gameplay/BP_TestGameInstance` (`GameplayStatics.GetGameInstance`) :!pure true))
      (set `PlayerController.bShowMouseCursor` true (`GameplayStatics.GetPlayerController` 0)))))

(fn `OnRep_HP`
  ;[1 1 1] 游戏失败判定
  (if (<= (`self.HP`) 0)
    (`GameplayStatics.SetGamePaused` true)
    (`/Game/Blueprint/Gameplay/BP_TestGameInstance.Defeat UI` (cast `/Game/Blueprint/Gameplay/BP_TestGameInstance` (`GameplayStatics.GetGameInstance`) :!pure true))
    (set `PlayerController.bShowMouseCursor` true (`GameplayStatics.GetPlayerController` 0))))

(fn `UserConstructionScript`)