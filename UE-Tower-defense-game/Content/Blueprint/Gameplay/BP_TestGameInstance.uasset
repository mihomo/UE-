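; Game instance that serves as a central spawner for the game's UI: start screen, runtime UI, tower attribute panel, and win and defeat screens.
; Each event creates its widget and adds it to the viewport.
; The tower panel is set up from a given tower floor and stored as RightUI on BP_Player.
; ClearUI removes any valid target widget and resets that RightUI reference.
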(event `GameBegin UI`
  ;[1 1 1] 创建游戏开始UI
  (bind _returnvalue (`|CreateWidget` "/Game/UI/WBP_Begin.WBP_Begin_C"))
  (`UserWidget.AddToViewport` _returnvalue 0))

(event `Runtime UI`
  ;[1 1 1] 创建运行时UI
  (bind _returnvalue (`|CreateWidget` "/Game/UI/RunTimeUI.RunTimeUI_C"))
  (`UserWidget.AddToViewport` _returnvalue 0))

(event `Clear UI`
  (params (`目标` :type "Widget Object Reference"))
  ;[1 1 1] 清除UI
  (`/Engine/EditorBlueprintResources/StandardMacros.IsValid` `目标`
    (:`Is Valid`
      (`Widget.RemoveFromParent` `目标`)
      (set `/Game/Item/BP_Player.Right UI` null (cast `/Game/Item/BP_Player` (`GameplayStatics.GetPlayerPawn` 0) :!pure true)))))

(event `TowerAtrribute UI`
  (params (RelateTowerFloor :type "/Game/Item/ItemBase/TowerFloorBase Object Reference"))
  ;[1 1 1] 创建塔属性UI
  (bind _returnvalue (`|CreateWidget` "/Game/UI/TowerAtrributeUI.TowerAtrributeUI_C"))
  (`UserWidget.AddToViewport` _returnvalue 0)
  (`/Game/UI/TowerAtrributeUI.Setting` _returnvalue RelateTowerFloor)
  (set `/Game/Item/BP_Player.Right UI` _returnvalue (cast `/Game/Item/BP_Player` (`GameplayStatics.GetPlayerPawn` 0) :!pure true)))

(event `Win UI`
  ;[1 1 1] 创建胜利UI
  (bind _returnvalue (`|CreateWidget` "/Game/UI/WBP_EndForWin.WBP_EndForWin_C"))
  (`UserWidget.AddToViewport` _returnvalue 0))

(event `Defeat UI`
  ;[1 1 1] 创建失败UI
  (bind _returnvalue (`|CreateWidget` "/Game/UI/WBP_EndForDefeat.WBP_EndForDefeat_C"))
  (`UserWidget.AddToViewport` _returnvalue 0))