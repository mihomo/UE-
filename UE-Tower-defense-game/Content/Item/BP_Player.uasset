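; Player Blueprint for a tower defense shooter that fires bullets, builds towers and collects pickups.
; SpawnTower_Server checks GameState resources, spawns a fire or ice tower on the floor base, links it and plays a build sound.
; Tick adds resources and updates game time each second, with an OnRep also adding resources.
; Capsule overlaps trigger BPI_Pick, while ChangeAttribute alters damage and fire rate, resetting them after a retriggerable delay.
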(event `self.ReceiveBeginPlay`
  (`GameplayStatics.GetActorOfClass` "/Script/Engine.CameraActor"))

(event `Spawn Tower_Server`
  (params (TowerClass :type Integer) (TowerFloorBase :type "/Game/Item/ItemBase/TowerFloorBase Object Reference") (TowerBuiltCount :type Integer))
  (bind _returnvalue (`self.GetTransform` TowerFloorBase))
  (bind _audio (`self.Audio`))
  (bind _asbp_test_game_state (cast `/Game/Blueprint/Gameplay/BP_TestGameState` (`GameplayStatics.GetGameState`) :!pure true))
  ;[1 1 1] 生成防御塔
  (if (not (< (+ (`/Game/Blueprint/Gameplay/BP_TestGameState.TPS Resources` (cast `/Game/Blueprint/Gameplay/BP_TestGameState` (`GameplayStatics.GetGameState`) :!pure true)) TowerBuiltCount) 0))
    (if (== TowerClass 0)
      (bind _returnvalue_2 (`|SpawnActorFromClass` "/Game/Item/TowerBase/Tower_Fire.Tower_Fire_C" _returnvalue "AdjustIfPossibleButAlwaysSpawn" "OverrideRootScale" TowerFloorBase null))
      (`/Game/Blueprint/Gameplay/BP_TestGameState.Change Atrribute` _asbp_test_game_state TowerBuiltCount 0 0 false false)
      (set `/Game/Item/ItemBase/TowerFloorBase.Relate Tower` _returnvalue_2 TowerFloorBase)
      (else
        (bind _returnvalue_3 (`|SpawnActorFromClass` "/Game/Item/TowerBase/Tower_Ice.Tower_Ice_C" _returnvalue "AdjustIfPossibleButAlwaysSpawn" "OverrideRootScale" TowerFloorBase null))
        (`/Game/Blueprint/Gameplay/BP_TestGameState.Change Atrribute` _asbp_test_game_state TowerBuiltCount 0 0 false false)
        (set `/Game/Item/ItemBase/TowerFloorBase.Relate Tower` _returnvalue_3 TowerFloorBase)))
    (`AudioComponent.SetSound` _audio "/Game/Music/Built_tower_01.Built_tower_01")
    (`AudioComponent.Play` _audio 0.0)))

(event `self.Capsule.OnComponentBeginOverlap`
  (params (OverlappedComponent :type "PrimitiveComponent Object Reference") (OtherActor :type "Actor Object Reference") (OtherComp :type "PrimitiveComponent Object Reference") (OtherBodyIndex :type Integer) (bFromSweep :type Boolean) (SweepResult :type "HitResult Structure (by ref)"))
  ;[1 1 1] 拾取东西
  (if (`KismetSystemLibrary.DoesImplementInterface` OtherActor "/Game/Blueprint/BPI_Pick.BPI_Pick_C")
    (message `/Game/Blueprint/BPI_Pick.Pick` OtherActor self)
    (`KismetSystemLibrary.PrintString` "Hello")))

(event `Change Attribute`
  (params (`Buttle Damage` :type Integer) (`Fire Speed` :type "Float (double-precision)"))
  ;[1 1 1] 更改攻击属性
  (if (not (`self.Power State`))
    (set `self.Bullet_A Damage` `Buttle Damage`)
    (set `self.Fire Speed` `Fire Speed`))
  (`KismetSystemLibrary.RetriggerableDelay` 10.0)
  (set `self.Bullet_A Damage` 50)
  (set `self.Fire Speed` 0.2))

(event `self.ReceiveTick`
  (params (DeltaSeconds :type "Float (single-precision)"))
  (bind _returnvalue (`KismetMathLibrary.FFloor64` (`self.GetGameTimeSinceCreation`)))
  (bind _asbp_test_game_state (cast `/Game/Blueprint/Gameplay/BP_TestGameState` (`GameplayStatics.GetGameState`) :!pure true))
  ;[1 1 1] 每秒增加资源
  (if (>= (- _returnvalue (`self.NewVar_0`)) 1)
    (set `self.NewVar_0` _returnvalue)
    (`/Game/Blueprint/Gameplay/BP_TestGameState.Change Atrribute` _asbp_test_game_state 5 0 0 false false)
    (set `/Game/Blueprint/Gameplay/BP_TestGameState.EnterMainLevelGameTime` _returnvalue _asbp_test_game_state)))

(event `Spawn Buttle`
  ;[1 1 1] 生成子弹
  (bind _returnvalue (`|SpawnActorFromClass` "/Game/Item/ItemBase/Bullet/Bullet_A.Bullet_A_C" (`KismetMathLibrary.MakeTransform` (`KismetMathLibrary.MakeVector` (.x (.location (`self.GetTransform`))) (.y (.location (`self.GetTransform`))) (+ (.z (.location (`self.GetTransform`))) 100.0)) (`KismetMathLibrary.MakeRotator` (.roll (`self.GetControlRotation`)) (+ (.pitch (`self.GetControlRotation`)) 5.0) (.yaw (`self.GetControlRotation`)))) "AdjustIfPossibleButAlwaysSpawn" "OverrideRootScale" null null))
  (`/Game/Item/ItemBase/BulletBase.Setting Damage` _returnvalue (`self.Bullet_A Damage`)))

(fn `OnRep_NewVar_0`
  (`/Game/Blueprint/Gameplay/BP_TestGameState.Change Atrribute` (cast `/Game/Blueprint/Gameplay/BP_TestGameState` (`GameplayStatics.GetGameState`) :!pure true) 1 0 0 false false))

(fn `UserConstructionScript`)