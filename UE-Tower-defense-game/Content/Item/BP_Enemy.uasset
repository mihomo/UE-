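; BP_Enemy is a networked enemy with a health bar that damages the team's home on contact.
; HP starts at MaxHP, and Tick pushes both values into the UI_HP widget.
; A server-only capsule overlap with Home destroys the enemy and subtracts health through BP_TestGameState.
; The HP RepNotify destroys it when HP drops below zero and decrements the GameState's enemy count.
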(event `self.ReceiveBeginPlay`
  ;[1 1 1] 初始化血量
  (set `self.HP` (`self.MaxHP`)))

(event `self.ReceiveTick`
  (params (DeltaSeconds :type "Float (single-precision)"))
  (bind _asui_hp (cast `/Game/UI/UI_HP` (`WidgetComponent.GetWidget` (`self.Widget`)) :!pure true))
  ;[1 1 1] 给血条UI传递血量
  (set `/Game/UI/UI_HP.HP` (`self.HP`) _asui_hp)
  (set `/Game/UI/UI_HP.MaxHP` (`self.MaxHP`) _asui_hp))

(event `self.Capsule.OnComponentBeginOverlap`
  (params (OverlappedComponent :type "PrimitiveComponent Object Reference") (OtherActor :type "Actor Object Reference") (OtherComp :type "PrimitiveComponent Object Reference") (OtherBodyIndex :type Integer) (bFromSweep :type Boolean) (SweepResult :type "HitResult Structure (by ref)"))
  ;[1 1 1] 进入家
  (if (`KismetSystemLibrary.IsServer`)
    (if (== (`GameplayStatics.GetObjectClass` OtherActor) "/Game/Item/ItemBase/Home.Home_C")
      (`self.K2_DestroyActor`)
      (`/Game/Blueprint/Gameplay/BP_TestGameState.Change Atrribute` (cast `/Game/Blueprint/Gameplay/BP_TestGameState` (`GameplayStatics.GetGameState`) :!pure true) 0 0 -10 false false))))

(fn `OnRep_HP`
  (if (< (`self.HP`) 0)
    (`self.K2_DestroyActor`)
    (`/Game/Blueprint/Gameplay/BP_TestGameState.Change Atrribute` (cast `/Game/Blueprint/Gameplay/BP_TestGameState` (`GameplayStatics.GetGameState`) :!pure true) 0 -1 0 false false)))

(fn `UserConstructionScript`)